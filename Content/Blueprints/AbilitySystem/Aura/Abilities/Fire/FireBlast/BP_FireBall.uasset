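; BP_FireBall is the FireBlast ability's projectile, which flies out and returns to explode near its ReturnToActor.
; On authority, two timelines lerp it forward to an apex, then back toward that actor's current location.
; Within ExplodeDistance it calls OnHit, damages nearby live players other than its owner with 45-degree knockback and death impulse, then destroys itself.
; Radial damage parameters are set only after the damage loop completes.
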(event EventBeginPlay)

(event Collision|EventActorBeginOverlap
  (params (OtherActor :type Actor%20Object%20Reference)))

(event EventTick
  (params (DeltaSeconds :type Float%20%28single-precision%29)))

(event EventStartOutgoingTimeline
  (bind _returnvalue (Components|GetOwner))
  (bind _array (Utilities|Array|MakeArray _returnvalue))
  (Networking|SwitchHasAuthority
    (:Authority
      (Variables|Default|SetInitialLocation (Transformation|GetActorLocation))
      (Variables|Default|SetApexLocation (+ (Variables|Default|GetInitialLocation) (* (Transformation|GetActorForwardVector) (Variables|Default|GetTravelDistance))))
      (bind _outgoingtrack (Timeline|OutgoingTimeline Play)
        (:Update
          (Transformation|SetActorLocation (Math|Vector|Lerp(Vector) (Variables|Default|GetInitialLocation) (Variables|Default|GetApexLocation) _outgoingtrack) false false))
        (:Finished
          (bind _returningtrack (Timeline|ReturningTimeline Play)
            (:Update
              (Transformation|SetActorLocation (Math|Vector|Lerp(Vector) (Variables|Default|GetApexLocation) (Transformation|GetActorLocation (Variables|Default|GetReturnToActor)) _returningtrack) false false)
              (if (CallFunction|IsWithinExplodeDistance)
                (Class|AuraProjectile|OnHit)
                (Utilities|Array|Add _array self)
                (bind _outoverlappingactors (Class|AuraAbilitySystemLibrary|GetLivePlayersWithinRadius 0 _array 0.0 (Transformation|GetActorLocation)))
                (bind _output_get (Variables|Default|SetOverlappingPlayers _outoverlappingactors))
                (for _array_element _output_get
                  (Class|AuraAbilitySystemLibrary|SetTargetEffectParamsASC (Variables|Default|GetExplosionDamageParams) (Ability|GetAbilitySystemComponent _array_element))
                  (Class|AuraAbilitySystemLibrary|SetKnockbackDirection (Variables|Default|GetExplosionDamageParams) (Math|Vector|GetForwardVector (Math|Rotator|MakeRotator (.roll (Math|Rotator|MakeRotfromX (- (Transformation|GetActorLocation _array_element) (Transformation|GetActorLocation)))) 45.0 (.yaw (Math|Rotator|MakeRotfromX (- (Transformation|GetActorLocation _array_element) (Transformation|GetActorLocation)))))) (Variables|Default|GetKnockbackDirectionMagnitude))
                  (Class|AuraAbilitySystemLibrary|SetDeathImpulseDirection (Variables|Default|GetExplosionDamageParams) (- (Transformation|GetActorLocation _array_element) (Transformation|GetActorLocation)) (Variables|Default|GetDeathImpulseMagnitude))
                  (Class|AuraAbilitySystemLibrary|ApplyDamageEffect (Variables|Default|GetExplosionDamageParams)))
                (Class|AuraAbilitySystemLibrary|SetIsRadialDamageEffectParam (Variables|Default|GetExplosionDamageParams) true 5e+01 3e+02 (Transformation|GetActorLocation))
                (Actor|DestroyActor)))))))))

(fn ConstructionScript)

(fn IsWithinExplodeDistance
  (return (<= (Math|Vector|VectorLength (- (Transformation|GetActorLocation) (Transformation|GetActorLocation (Variables|Default|GetReturnToActor)))) (Variables|Default|GetExplodeDistance))))