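; Arcane Shards gameplay ability that shows a magic circle, then on press raises damaging shards around the targeted ground point.
; It spawns a point collection at the cursor hit for randomly rotated ground points and plays the cast montage.
; The montage event commits cost and starts a looping timer, spawning one shard cue per tick with radial damage and pitched outward knockback.
; Shard count follows ability level up to a cap, then cooldown commits.
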(event Custom|Spawn%20Shard
  (bind _returnvalue (Ability|GetAvatarActorfromActorInfo))
  (if (< (Variables|Default|GetCount) (Math|Integer|Min(Integer) (Ability|GetAbilityLevel) (Variables|Default|GetMaxNumShards)))
    (Variables|Default|SetShardSpawnLocation (Transformation|GetWorldLocation (Utilities|Array|Get(acopy) (Variables|Default|GetGroundPoints) (Variables|Default|GetCount))))
    (bind _outoverlappingactors (Class|AuraAbilitySystemLibrary|GetLivePlayersWithinRadius _returnvalue (Utilities|Array|MakeArray _returnvalue) (Variables|Default|GetRadialDamageOuterRadius) (Variables|Default|GetShardSpawnLocation)))
    (bind _output_get (Variables|Default|SetOverlappingPlayers _outoverlappingactors))
    (for _array_element _output_get
      (Class|AuraAbilitySystemLibrary|ApplyDamageEffect (Class|AuraDamageGameplayAbility|MakeDamageEffectParamsfromClassDefaults _array_element (Variables|Default|GetShardSpawnLocation) true (- (Transformation|GetActorLocation _array_element) (Variables|Default|GetShardSpawnLocation)) true (- (Transformation|GetActorLocation _array_element) (Variables|Default|GetShardSpawnLocation)) true 45.0)))
    (Math|Integer|IncrementInt (Variables|Default|GetCount)
      (:%20%20
        (Class|GameplayAbility|ExecuteGameplayCuewithParams "(TagName=\"GameplayCue.ArcaneShards\")" (Ability|GameplayCue|MakeGameplayCueParameters :Location (Variables|Default|GetShardSpawnLocation)))))
    (else
      (Utilities|Time|ClearandInvalidateTimerbyHandle (Variables|Default|GetShardSpawnTimer))
      (Actor|DestroyActor (Variables|Default|GetPointCollection))
      (Ability|CommitAbilityCooldown false)
      (Ability|EndAbility))))

(event Ability|EventActivateAbility
  (bind _returnvalue (Class|GameplayAbility|CheckAbilityCost))
  (if _returnvalue
    (Utilities|FlowControl|Sequence
      (:then_0
        (Class|PlayerInterface|ShowMagicCircle(Message) (Ability|GetAvatarActorfromActorInfo) 0))
      (:then_1
        (Ability|Tasks|WaitInputPress false
          (:OnPress
            (bind _datahandle (|TargetDataUnderMouse)
              (:ValidData
                (bind _output_get (Variables|Default|SetMouseHitLocation (.ImpactPoint (Collision|BreakHitResult (Ability|TargetData|GetHitResultfromTargetData _datahandle)))))
                (bind _returnvalue_2 (Game|SpawnActorfromClass "/Game/Blueprints/AbilitySystem/Aura/Abilities/Arcane/ArcaneShards/BP_PointCollection.BP_PointCollection_C" (Math|Transform|MakeTransform _output_get "0, 0, 0" "1.000000,1.000000,1.000000") "AlwaysSpawn" "MultiplyWithRoot" 0 0))
                (bind _output_get_2 (Variables|Default|SetPointCollection _returnvalue_2))
                (Variables|Default|SetGroundPoints (Class|PointCollection|GetGroundPoints _output_get_2 (Variables|Default|GetMouseHitLocation) (Variables|Default|GetMaxNumShards) (Math|Random|RandomFloatinRange 0.0 3.6e+02)))
                (Class|CombatInterface|UpdateFacingTarget(Message) (Ability|GetAvatarActorfromActorInfo) (Variables|Default|GetMouseHitLocation))
                (|PlayMontageandWaitProxy "None" "/Game/Assets/Characters/Aura/Animations/Abilities/AM_CastArcaneShards.AM_CastArcaneShards" 1.0 "None" false 1.0 0.0 false
                  (:then
                    (Ability|Tasks|WaitGameplayEvent "(TagName=\"Event.Montage.ArcaneShards\")" 0 true
                      (:EventReceived
                        (bind _returnvalue_3 (Utilities|Time|SetTimerbyEvent (delegate Custom|Spawn%20Shard) (Variables|Default|GetShardSpawnDeltaTime) true))
                        (Variables|Default|SetShardSpawnTimer _returnvalue_3)
                        (CallFunction|SpawnShard)
                        (Class|PlayerInterface|HideMagicCircle(Message) (Ability|GetAvatarActorfromActorInfo))
                        (Ability|CommitAbilityCost false)))))))))))))